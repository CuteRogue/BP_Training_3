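; Game mode that runs endless enemy waves of growing size and starts a looping wind ambience on BeginPlay.
; SetupNewWave starts a looping timer, by function name, that spawns BP_Enemy at random TargetPoints until EnemiesRemaining runs out.
; RegisterEnemyDeath removes enemies from the tracked array and ends the wave once none are alive or left to spawn.
; EndWave waits briefly, multiplies the next wave's enemy count, and restarts the cycle.
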(event `self.ReceiveBeginPlay`
  (`GameplayStatics.PlaySound2D` "/Game/Sounds/AmbientLoops/Stereo/WindSteady_Loop_Stereo_Cue.WindSteady_Loop_Stereo_Cue" 1.0 1.0 0.0 null null)
  (`KismetSystemLibrary.Delay` 2.0)
  (`self.Setup New Wave`))

(event `Spawn Wave`
  (`self.Spawn Enemy`))

(event `End Wave`
  (`KismetSystemLibrary.Delay` 2.0)
  (`self.Increase Difficulty Multiplier`)
  (`self.Setup New Wave`))

(fn `Get Random Spawn Point`
  (returns (Output :type "TargetPoint Object Reference"))
  (bind _outactors (`GameplayStatics.GetAllActorsOfClass` "/Script/Engine.TargetPoint"))
  (return (`|GetArrayItem` _outactors (`KismetMathLibrary.RandomIntegerInRange` 0 (`KismetArrayLibrary.Array_LastIndex` _outactors)))))

(fn `Increase Difficulty Multiplier`
  (bind _output_get (set `self.Wave Difficulty` (`KismetMathLibrary.Round` (* (`self.Wave Difficulty`) (`self.Multiplier Per Wave`)))))
  (set `self.Enemies Remaining` _output_get))

(fn `Is Wave Completed`
  (returns (ReturnValue :type Boolean))
  (return (and (<= (`KismetArrayLibrary.Array_Length` (`self.Enemies`)) 0) (<= (`self.Enemies Remaining`) 0))))

(fn `Register Enemy Death`
  (params (Enemy :type "/Game/Blueprints/AI/BP_Enemy Object Reference"))
  (`KismetArrayLibrary.Array_RemoveItem` (`self.Enemies`) Enemy)
  (if (`self.Is Wave Completed`)
    (`self.End Wave`)))

(fn `Setup New Wave`
  (`/Engine/EditorBlueprintResources/StandardMacros.IncrementInt` (`self.Current Wave`)
    (:`  `
      (`KismetSystemLibrary.K2_SetTimer` null "Spawn Wave" 1.0 true))))

(fn `Spawn Enemy`
  (bind _output (`self.Get Random Spawn Point`))
  (`/Engine/EditorBlueprintResources/StandardMacros.IsValid` _output
    (:`Is Valid`
      (bind _returnvalue (`|SpawnActorFromClass` "/Game/Blueprints/AI/BP_Enemy.BP_Enemy_C" (`self.GetTransform` _output) "Undefined" "MultiplyWithRoot" null null))
      (`/Engine/EditorBlueprintResources/StandardMacros.IsValid` _returnvalue
        (:`Is Valid`
          (`KismetArrayLibrary.Array_Add` (`self.Enemies`) _returnvalue)
          (bind _result (`/Engine/EditorBlueprintResources/StandardMacros.DecrementInt` (`self.Enemies Remaining`))
            (:`  `
              (if (<= _result 0)
                (`KismetSystemLibrary.K2_ClearTimer` null "Spawn Wave")))))))))

(fn `UserConstructionScript`)