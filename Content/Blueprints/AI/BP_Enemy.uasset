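; BP_Enemy is an AI enemy that chases the player, plays a melee attack montage in range, and handles its own death.
; A repeating AIMoveTo drives pursuit, while Tick checks distance and suspends movement during attacks.
; DamagePlayer applies damage but is not called within this Blueprint.
; Damage plays an impact sound and reduces health; death disables collision and movement, credits the BP_Marine killer, notifies BP_GameMode, then destroys the actor.
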(event `self.ReceiveBeginPlay`
  (`|AIMoveTo` self (0.0 0.0 0.0) (`GameplayStatics.GetPlayerCharacter` 0) :!label _label
    (:`OnSuccess`
      (`KismetSystemLibrary.Delay` 0.2 :!label _label_2)
      (goto _label))
    (:`OnFail`
      (if (`self.Is Alive`)
        (goto _label_2)))))

(event `self.ReceiveTick`
  (params (DeltaSeconds :type "Float (single-precision)"))
  (bind _charactermovement (`self.CharacterMovement`))
  (if (and (`self.Is In Range`) (not (`self.Is Attacking`)) (`self.Is Alive`))
    (`ActorComponent.Deactivate` _charactermovement)
    (`|PlayMontage` (`self.Mesh`) "/Game/Characters/Enemy_Great_Spider/Animations/AM_Attack.AM_Attack"
      (:`OnCompleted`
        (`ActorComponent.Activate` _charactermovement false)))))

(event `self.ReceiveAnyDamage`
  (params (Damage :type "Float (single-precision)") (DamageType :type "DamageType Object Reference") (InstigatedBy :type "Controller Object Reference") (DamageCauser :type "Actor Object Reference"))
  (`GameplayStatics.PlaySoundAtLocation` "/Game/Sounds/FoleyFlesh/Mono/FoleyFlesh_Impact_Cue.FoleyFlesh_Impact_Cue" (`self.K2_GetActorLocation`) (struct) 1.0 1.0 0.0 null null null null)
  (if (`self.Is Alive`)
    (bind _remaining_health (`self.Decrease Health` Damage))
    (if (<= _remaining_health 0.0)
      (`self.Setup Before Death`
        (:`Completed`
          (set `self.Dead` true)
          (`self.Setup After Death`
            (:`Completed`
              (bind _asbp_marine (cast `/Game/Blueprints/Pawns/BP_Marine` DamageCauser))
              (`/Game/Blueprints/Pawns/BP_Marine.Increase Kiils` _asbp_marine)
              (bind _asbp_game_mode (cast `/Game/Blueprints/GameModes/BP_GameMode` (`GameplayStatics.GetGameMode`)))
              (`/Game/Blueprints/GameModes/BP_GameMode.Register Enemy Death` _asbp_game_mode self)
              (`KismetSystemLibrary.Delay` 2.0)
              (`self.K2_DestroyActor`))))))))

(fn `Damage Player`
  (`GameplayStatics.ApplyDamage` (`GameplayStatics.GetPlayerCharacter` 0) (`self.Base Damage`)))

(fn `Decrease Health`
  (params (Damage :type "Float (double-precision)"))
  (returns (`Remaining Health` :type "Float (double-precision)"))
  (bind _output_get (set `self.Health` (`KismetMathLibrary.FClamp` (- (`self.Health`) Damage) 0.0 (`self.Max Health`))))
  (return _output_get))

(fn `Is Alive`
  (returns (ReturnValue :type Boolean))
  (return (not (`self.Dead`))))

(fn `Is Attacking`
  (returns (ReturnValue :type Boolean))
  (bind _returnvalue (`SkeletalMeshComponent.GetAnimInstance` (`self.Mesh`)))
  (`/Engine/EditorBlueprintResources/StandardMacros.IsValid` _returnvalue
    (:`Is Valid`
      (return (`AnimInstance.Montage_IsPlaying` _returnvalue "/Game/Characters/Enemy_Great_Spider/Animations/AM_Attack.AM_Attack")))
    (:`Is Not Valid`
      (return false))))

(fn `Is In Range`
  (returns (ReturnValue :type Boolean))
  (return (<= (`self.GetDistanceTo` (`GameplayStatics.GetPlayerCharacter` 0)) (`self.Attack Range`))))

(fn `UserConstructionScript`)