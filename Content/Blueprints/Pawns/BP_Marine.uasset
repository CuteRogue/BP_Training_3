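; Player marine character for a shooter, with world-axis movement, yaw-only aiming, health, a kill counter and a HUD.
; Enhanced Input drives movement and aim; stick look sets yaw directly, while Tick interpolates toward the mouse-axis angle.
; Firing runs a looping timer of muzzle line traces that apply damage and spawn impacts.
; Damage leads to death, which disables control; leaving the play area adds a red fade, warning sound and timed damage.
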(event `self.ReceiveBeginPlay`
  (`self.Setup Enhanced Input`)
  (`self.Setup HUD`))

(event `self.ReceiveTick`
  (params (DeltaSeconds :type "Float (single-precision)"))
  (bind _returnvalue (`GameplayStatics.GetPlayerController` 0))
  (bind (_mouse_axis_x _mouse_axis_y) (`KismetMathLibrary.BreakVector2D` (`self.Mouse Axis`)))
  (`Controller.SetControlRotation` _returnvalue (`KismetMathLibrary.RInterpTo` (`self.K2_GetActorRotation` _returnvalue) (`KismetMathLibrary.MakeRotator` 0.0 0.0 (`KismetMathLibrary.DegAtan2` _mouse_axis_x _mouse_axis_y)) (`GameplayStatics.GetWorldDeltaSeconds`) (`self.Mouse Smoothing`)))
  (`self.Fire Weapon Trace Loop`))

(event `EnhancedInput|/Game/Input/IA_Look`
  (params (ActionValue :type "Vector2D Structure") (ElapsedSeconds :type "Float (double-precision)") (TriggeredSeconds :type "Float (double-precision)") (InputAction :type "InputAction Object Reference" :default "/Game/Input/IA_Look.IA_Look"))
  (:`Triggered`
    (`Controller.SetControlRotation` (`GameplayStatics.GetPlayerController` 0) (`KismetMathLibrary.MakeRotator` 0.0 0.0 (`KismetMathLibrary.DegAtan2` ActionValue_X (* ActionValue_Y -1.0))))))

(event `EnhancedInput|/Game/Input/IA_Move`
  (params (ActionValue :type "Vector2D Structure") (ElapsedSeconds :type "Float (double-precision)") (TriggeredSeconds :type "Float (double-precision)") (InputAction :type "InputAction Object Reference" :default "/Game/Input/IA_Move.IA_Move"))
  (:`Triggered`
    (`self.AddMovementInput` (`KismetMathLibrary.MakeVector` ActionValue_Y ActionValue_X))))

(event `EnhancedInput|/Game/Input/IA_MouseLook`
  (params (ActionValue :type "Vector2D Structure") (ElapsedSeconds :type "Float (double-precision)") (TriggeredSeconds :type "Float (double-precision)") (InputAction :type "InputAction Object Reference" :default "/Game/Input/IA_MouseLook.IA_MouseLook"))
  (:`Triggered`
    (set `self.Mouse Axis` ActionValue)))

(event `EnhancedInput|/Game/Input/IA_Fire`
  (params (ActionValue :type Boolean) (ElapsedSeconds :type "Float (double-precision)") (TriggeredSeconds :type "Float (double-precision)") (InputAction :type "InputAction Object Reference" :default "/Game/Input/IA_Fire.IA_Fire"))
  (:`Started`
    (`self.Start Fire Weapon`))
  (:`Completed`
    (`self.Stop Fire Weapon`)))

(event `self.ReceiveAnyDamage`
  (params (Damage :type "Float (single-precision)") (DamageType :type "DamageType Object Reference") (InstigatedBy :type "Controller Object Reference") (DamageCauser :type "Actor Object Reference"))
  (if (`self.Is Alive`)
    (bind _remaining_health (`self.Decrease Health` Damage))
    (if (<= _remaining_health 0.0)
      (`self.Setup Before Death`
        (:`Completed`
          (set `self.Dead` true))))))

(event `Decrease Health Interval`
  (`GameplayStatics.ApplyDamage` self (`self.Ouside Play Area Damage`)))

(fn `Decrease Health`
  (params (Damage :type "Float (double-precision)"))
  (returns (`Remaining Health` :type "Float (double-precision)"))
  (bind _output_get (set `self.Health` (- (`self.Health`) Damage)))
  (return (`KismetMathLibrary.FClamp` _output_get 0.0 (`self.Max Health`))))

(fn `Fire Weapon Trace Loop`
  (if (`self.Is Firing`)
    _))

(fn `Increase Kiils`
  (set `self.Kills` (+ (`self.Kills`) 1)))

(fn `Inside Play Area`
  (bind _outside_play_area_sound (`self.Outside Play Area Sound`))
  (set `self.In Play Area` true)
  (`/Engine/EditorBlueprintResources/StandardMacros.IsValid` _outside_play_area_sound
    (:`Is Valid`
      (`AudioComponent.Stop` _outside_play_area_sound)
      (`PlayerCameraManager.StopCameraFade` (`GameplayStatics.GetPlayerCameraManager` 0))
      (`KismetSystemLibrary.K2_ClearTimer` null "Decrease Health Interval"))))

(fn `Is Alive`
  (returns (ReturnValue :type Boolean))
  (return (not (`self.Dead`))))

(fn `Is Health Full`
  (returns (ReturnValue :type Boolean))
  (return (>= (`self.Health`) (`self.Max Health`))))

(fn `Outside Play Area`
  (set `self.In Play Area` false)
  (bind _returnvalue (`GameplayStatics.SpawnSound2D` "/Game/Sounds/InterfaceAudio/Stereo/UI_LowHealth_Loop_Stereo.UI_LowHealth_Loop_Stereo" 1.0 1.0 0.0 null))
  (set `self.Outside Play Area Sound` _returnvalue)
  (`PlayerCameraManager.StartCameraFade` (`GameplayStatics.GetPlayerCameraManager` 0) 0.0 0.5 1.0 (struct :`R` 1.0 :`B` 0.055031 :`A` 1.0) false true)
  (`KismetSystemLibrary.K2_SetTimer` null "Decrease Health Interval" 1.0 true))

(fn `Recover Health`
  (params (Amount :type "Float (double-precision)"))
  (set `self.Health` (`KismetMathLibrary.FClamp` (+ Amount (`self.Health`)) 0.0 (`self.Max Health`))))

(fn `Setup Enhanced Input`
  (bind _asplayer_controller (cast `PlayerController` (`self.GetController`)))
  (bind _returnvalue (pcsubsystem `EnhancedInputLocalPlayerSubsystem` _asplayer_controller))
  (`/Engine/EditorBlueprintResources/StandardMacros.IsValid` _returnvalue
    (:`Is Valid`
      (`EnhancedInputSubsystemInterface.AddMappingContext` _returnvalue "/Game/Input/IMC_Input.IMC_Input" 0 (struct)))))

(fn `Setup HUD`
  (bind _returnvalue (`|CreateWidget` "/Game/UI/WBP_PlayerHUD.WBP_PlayerHUD_C" null self))
  (`UserWidget.AddToViewport` _returnvalue 0))

(fn `Spawn Impact Hit`
  (params (`Spawn Point` :type "Vector Structure"))
  (`GameplayStatics.SpawnEmitterAtLocation` "/Game/Effects/Weapons/Impacts/P_AssaultRifle_IH.P_AssaultRifle_IH" `Spawn Point`))

(fn `Start Fire Weapon`
  (if (and (`self.Is Alive`) (not (`self.Is Firing`)))
    (`ActorComponent.Activate` (`self.P_AssaultRifle_MF`) false)
    (bind _returnvalue (`GameplayStatics.SpawnSound2D` "/Game/Sounds/Weapon_AssaultRifle/Stereo/RifleFireLoopCue.RifleFireLoopCue" 1.0 1.0 0.0 null))
    (set `self.Weapon Fire Sound` _returnvalue)
    (set `self.Is Firing` true)
    (`self.Weapon Trace`)
    (`KismetSystemLibrary.K2_SetTimer` null "Weapon Trace" (`self.Fire Delay`) true)))

(fn `Stop Fire Weapon`
  (bind _weapon_fire_sound (`self.Weapon Fire Sound`))
  (if (`self.Is Firing`)
    (`ActorComponent.Deactivate` (`self.P_AssaultRifle_MF`))
    (`/Engine/EditorBlueprintResources/StandardMacros.IsValid` _weapon_fire_sound
      (:`Is Valid`
        (`AudioComponent.Stop` _weapon_fire_sound)
        (`GameplayStatics.SpawnSound2D` "/Game/Sounds/Weapon_AssaultRifle/Stereo/RifleFireEndCue.RifleFireEndCue" 1.0 1.0 0.0 null)
        (set `self.Is Firing` false)
        (`KismetSystemLibrary.K2_ClearTimer` null "Weapon Trace")))))

(fn `UserConstructionScript`)

(fn `Weapon Trace`
  (bind _returnvalue (`SceneComponent.GetSocketLocation` (`self.Rifle`) "MuzzleFlash"))
  (bind _outhit (`KismetSystemLibrary.LineTraceSingle` _returnvalue (+ _returnvalue (* (`KismetMathLibrary.GetForwardVector` (`self.GetControlRotation`)) (`self.Weapon Range`))) "TraceTypeQuery1"))
  (bind (_bblockinghit _binitialoverlap _time _distance _location _impactpoint _normal _impactnormal _physmat _hitactor) (`GameplayStatics.BreakHitResult` _outhit))
  (if _bblockinghit
    (`GameplayStatics.ApplyDamage` _hitactor (`self.Weapon Damage`) null self)
    (`self.Spawn Impact Hit` _impactpoint)))